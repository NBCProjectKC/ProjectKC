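; Cooking pot actor that animates its lid as cooking starts and completes.
; BeginPlay derives an open position above the lid's initial closed position and hides it.
; Cooking start shows the lid and plays a timeline, while completion reverses it, then hides the lid after a delay unless cooking restarts.
; The timeline's interpolated location passes through a rotation round trip, reducing it to a unit vector.
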(event EventBeginPlay
  (bind _output_get (Variables|Default|SetLidClosedLocation (Variables|/Script/Engine.SceneComponent|GetRelativeLocation (Variables|Default|GetLidMesh))))
  (bind _output_get_2 (Variables|Default|SetLidOpenLocation (+ _output_get (Math|Vector|MakeVector 0.0 0.0 (Variables|Default|GetLidLiftHeight)))))
  (Transformation|SetRelativeLocation (Variables|Default|GetLidMesh) _output_get_2 false false)
  (Rendering|SetVisibility (Variables|Default|GetLidMesh) false false))

(event Collision|EventActorBeginOverlap
  (params (OtherActor :type Actor%20Object%20Reference)))

(event EventTick
  (params (DeltaSeconds :type Float%20%28single-precision%29)))

(event EventOnCookingStarted
  (Variables|Default|SetbPendingLidHide false)
  (Transformation|SetRelativeLocation (Variables|Default|GetLidMesh) (Variables|Default|GetLidOpenLocation) false false)
  (Rendering|SetVisibility (Variables|Default|GetLidMesh) true false)
  (Components|Timeline|PlayfromStart (Variables|Default|GetTL_LidMove)))

(event EventOnCookingCompleted
  (Variables|Default|SetbPendingLidHide true)
  (Components|Timeline|ReversefromEnd (Variables|Default|GetTL_LidMove)))

(fn ConstructionScript)