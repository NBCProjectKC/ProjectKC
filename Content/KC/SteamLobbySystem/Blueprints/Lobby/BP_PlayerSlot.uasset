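; BP_PlayerSlot is a clickable player slot actor in the Steam lobby.
; Clicking it asks the local KCLobbyPlayerController to request a move to its SlotIndex.
; On slot state changes, Empty, Occupied and Ready share one cylinder material, while Closed applies a different one and disables Box collision.
; No branch in this graph re-enables that collision.
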(event MouseInput|EventActorOnClicked
  (params (ButtonPressed :type Key%20Structure :default "None"))
  ;[0.15 0.05968 0.04045 0.5] 슬롯 클릭
  (bind _askclobby_player_controller (Utilities|Casting|CastToKCLobbyPlayerController (Game|GetPlayerController 0)))
  (Class|KCLobbyPlayerController|ROSRequestMovetoSlot _askclobby_player_controller (Variables|Default|GetSlotIndex)))

(event EventOnSlotStateChanged
  (params (NewState :type EKCLobbySlotStateType%20Enum :default "Empty"))
  ;[0.1111 0.15 0.03381 0.5] 슬롯 활성화/비활성화 시 상태 다르게 적용
  (switch Utilities|FlowControl|Switch|SwitchonEKCLobbySlotStateType NewState
    (:Empty
      (Rendering|Material|SetMaterial (Variables|Default|GetCylinder) 0 "/Engine/BasicShapes/BasicShapeMaterial.BasicShapeMaterial" :!label _label))
    (:Occupied
      (goto _label))
    (:Ready
      (goto _label))
    (:Closed
      (Rendering|Material|SetMaterial (Variables|Default|GetCylinder) 0 "/Engine/BasicShapes/BasicShapeMaterial_Inst.BasicShapeMaterial_Inst")
      (Collision|SetCollisionEnabled (Variables|Default|GetBox) "NoCollision"))))

(fn ConstructionScript)