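; BP_MicorwaveArena is a microwave arena level actor with a spinning visual root that carries pot actors around its center.
; BeginPlay caches each pot's offset from that root.
; While IsRotating is set, Tick accumulates a wrapped yaw angle and turns the root on every instance running it.
; Only the authority repositions pots, rotating their cached offsets around world Z without sweeping or changing their orientation, rather than attaching them.
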(event EventBeginPlay
  (Utilities|Array|Clear (Variables|Default|GetPotInitialOffsets))
  (for (_array_element _array_index) (Variables|Default|GetPotActors)
    (Utilities|IsValid _array_element
      (:Is%20Valid
        (Utilities|Array|SetArrayElem (Variables|Default|GetPotInitialOffsets) _array_index (- (Transformation|GetActorLocation _array_element) (Transformation|GetWorldLocation (Variables|Default|GetRotatingVisualRoot))) true)))))

(event Collision|EventActorBeginOverlap
  (params (OtherActor :type Actor%20Object%20Reference)))

(event EventTick
  (params (DeltaSeconds :type Float%20%28single-precision%29))
  (if (Variables|Default|GetbIsRotating)
    (bind _output_get (Variables|Default|SetCurrentRotationAngle (Math|Float|%(Float) (+ (* DeltaSeconds (Variables|Default|GetRotationSpeed)) (Variables|Default|GetCurrentRotationAngle)) 3.6e+02)))
    (Transformation|SetRelativeRotation (Variables|Default|GetRotatingVisualRoot) (Math|Rotator|MakeRotator 0.0 0.0 _output_get) false false)
    (Networking|SwitchHasAuthority
      (:Authority
        (for (_array_element _array_index) (Variables|Default|GetPotActors)
          (Utilities|IsValid _array_element
            (:Is%20Valid
              (Transformation|SetActorLocation _array_element (+ (Math|Vector|RotateVectorAroundAxis (Utilities|Array|Get(acopy) (Variables|Default|GetPotInitialOffsets) _array_index) (Variables|Default|GetCurrentRotationAngle) "0.000000,0.000000,1.000000") (Transformation|GetWorldLocation (Variables|Default|GetRotatingVisualRoot))) false false))))))))

(fn ConstructionScript)